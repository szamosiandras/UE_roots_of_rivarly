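; Interactive spline actor that builds a chain of spline meshes and grows when any segment is clicked.
; The construction script creates one mesh per point pair, offset sideways by half its bounds, and binds mouse events.
; Clicking appends a point along local X from the last one, with a new bound segment; hovering swaps the segment's material.
; BeginPlay enables cursor events and spline display; trace-spawn and other experiments are disconnected.
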(event `self.ReceiveBeginPlay`
  (bind _returnvalue (`GameplayStatics.GetPlayerController` 0))
  (`|ExecutionSequence`
    (:`then_0`
      (set `PlayerController.bEnableMouseOverEvents` true _returnvalue)
      (set `PlayerController.bEnableClickEvents` true _returnvalue)
      (set `PlayerController.bShowMouseCursor` true _returnvalue)
      (`KismetSystemLibrary.ExecuteConsoleCommand` "show splines" null))))

(event `self.SplineMeshComponent.OnBeginCursorOver`
  (params (TouchedComponent :type "PrimitiveComponent Object Reference"))
  (`KismetSystemLibrary.PrintString` "Mesh cursor over"))

(event `self.Spline.OnBeginCursorOver`
  (params (TouchedComponent :type "PrimitiveComponent Object Reference"))
  (`KismetSystemLibrary.PrintString` "Spline cursor over"))

(event `SplineMeshClicked`
  (params (TouchedComponent :type "PrimitiveComponent Object Reference") (ButtonPressed :type "Key Structure" :default "None"))
  (`KismetSystemLibrary.PrintString` "Clicked")
  (bind _addedsplinemesh (`self.AddSplinePoint`))
  (add `PrimitiveComponent.OnBeginCursorOver` _addedsplinemesh (`|CreateDelegate` :!event `SplineMeshCursorOverBegin`))
  (add `PrimitiveComponent.OnClicked` _addedsplinemesh (`|CreateDelegate` :!event `SplineMeshClicked`))
  (add `PrimitiveComponent.OnEndCursorOver` _addedsplinemesh (`|CreateDelegate` :!event `SplineMeshCursorOverEnd`)))

(event `SplineMeshCursorOverBegin`
  (params (TouchedComponent :type "PrimitiveComponent Object Reference"))
  (`KismetSystemLibrary.PrintString` "Mouse Over Start")
  (`PrimitiveComponent.SetMaterial` TouchedComponent 0 "/Game/StarterContent/Materials/M_Metal_Gold.M_Metal_Gold"))

(event `SplineMeshCursorOverEnd`
  (params (TouchedComponent :type "PrimitiveComponent Object Reference"))
  (`KismetSystemLibrary.PrintString` "Mouse Over End")
  (`PrimitiveComponent.SetMaterial` TouchedComponent 0 "/Game/StarterContent/Materials/M_Basic_Wall.M_Basic_Wall"))

(fn `AddSplinePoint`
  (returns (AddedSplineMesh :type "SplineMeshComponent Object Reference"))
  (bind (_start_point _start_tangent _end_point _end_tangent) (`self.GetSplineLatsTwoPoints`))
  (bind _spline (`self.Spline`))
  (bind (_returnvalue_x _returnvalue_y _returnvalue_z) (`KismetMathLibrary.BreakVector` (`SplineComponent.GetLocationAtSplinePoint` _spline (- (`SplineComponent.GetNumberOfSplinePoints` _spline) 1) "Local")))
  (`KismetSystemLibrary.PrintString` "click")
  (`SplineComponent.AddSplinePoint` _spline (`KismetMathLibrary.MakeVector` (+ _returnvalue_x 100.0) _returnvalue_y _returnvalue_z) "Local" true)
  (bind _returnvalue (`AddComponent|NODE_AddSplineMeshComponent-5`))
  (`KismetArrayLibrary.Array_Add` (`self.SplineMeshComponents`) _returnvalue)
  (`SplineMeshComponent.SetForwardAxis` _returnvalue "Y" true)
  (`SceneComponent.K2_AttachToComponent` _returnvalue (`self.Spline`) "None" "KeepRelative" "KeepRelative" "KeepRelative" true)
  (bind _spliemeshsizes_x (`KismetMathLibrary.BreakVector` (`self.GetSplineMeshHalfSizes` _returnvalue)))
  (`SplineMeshComponent.SetStartAndEnd` _returnvalue (+ _start_point (`KismetMathLibrary.MakeVector` 0.0 _spliemeshsizes_x)) _start_tangent (+ _end_point (`KismetMathLibrary.MakeVector` 0.0 (* _spliemeshsizes_x 1.0))) _end_tangent true)
  (`KismetSystemLibrary.PrintString` (`KismetStringLibrary.Conv_IntToString` (`KismetArrayLibrary.Array_Length` (`self.SplineMeshComponents`))))
  (return _returnvalue))

(fn `GetSplineLatsTwoPoints`
  (returns (`Start Point` :type "Vector Structure") (`Start Tangent` :type "Vector Structure") (`End Point` :type "Vector Structure") (`End Tangent` :type "Vector Structure"))
  (bind _spline (`self.Spline`))
  (bind _returnvalue (`SplineComponent.GetNumberOfSplinePoints` _spline))
  (bind _returnvalue_2 (- _returnvalue 1))
  (bind _returnvalue_3 (- _returnvalue 2))
  (return (`SplineComponent.GetLocationAtSplinePoint` _spline _returnvalue_3 "Local") (`SplineComponent.GetTangentAtSplinePoint` _spline _returnvalue_3 "Local") (`SplineComponent.GetLocationAtSplinePoint` _spline _returnvalue_2 "Local") (`SplineComponent.GetTangentAtSplinePoint` _spline _returnvalue_2 "Local")))

(fn `GetSplineMeshHalfSizes`
  (params (SplineMesh :type "SplineMeshComponent Object Reference"))
  (returns (SplieMeshSizes :type "Vector Structure"))
  (bind (_min _max) (`StaticMeshComponent.GetLocalBounds` SplineMesh))
  (return (/ (- _min _max) (2.0 2.0 2.0))))

(fn `UserConstructionScript`
  (bind _spline (`self.Spline`))
  (bind _spline_2 (`self.Spline`))
  (for _index (range (+ (- (`SplineComponent.GetNumberOfSplinePoints` (`self.Spline`)) 2) 1))
    (bind _returnvalue (`AddComponent|NODE_AddSplineMeshComponent-0`))
    (`KismetArrayLibrary.Array_Add` (`self.SplineMeshComponents`) _returnvalue)
    (bind _output_get (set `self.SplineMeshComponent` _returnvalue))
    (`SplineMeshComponent.SetForwardAxis` _output_get "Y" true)
    (`SceneComponent.K2_AttachToComponent` _output_get (`self.Spline`) "None" "KeepRelative" "KeepRelative" "KeepRelative" true)
    (bind _spliemeshsizes_x (`KismetMathLibrary.BreakVector` (`self.GetSplineMeshHalfSizes` _output_get)))
    (bind _returnvalue_2 (+ _index 1))
    (`SplineMeshComponent.SetStartAndEnd` _output_get (+ (`SplineComponent.GetLocationAtSplinePoint` _spline_2 _index "Local") (`KismetMathLibrary.MakeVector` 0.0 _spliemeshsizes_x)) (`SplineComponent.GetTangentAtSplinePoint` _spline_2 _index "Local") (+ (`SplineComponent.GetLocationAtSplinePoint` _spline _returnvalue_2 "Local") (`KismetMathLibrary.MakeVector` 0.0 _spliemeshsizes_x)) (`SplineComponent.GetTangentAtSplinePoint` _spline _returnvalue_2 "Local") true)
    (add `PrimitiveComponent.OnClicked` _returnvalue (`|CreateDelegate` :!event `SplineMeshClicked`))
    (add `PrimitiveComponent.OnBeginCursorOver` _returnvalue (`|CreateDelegate` :!event `SplineMeshCursorOverBegin`))
    (add `PrimitiveComponent.OnEndCursorOver` _returnvalue (`|CreateDelegate` :!event `SplineMeshCursorOverEnd`))))