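; BP_BranchFactory is a clickable, growable tree branch built from spline meshes along a spline.
; Hovering brightens it; clicking retargets the scene capture and opens a details widget with Build and HotRes upgrade controls.
; Building adds a spline point along the Arrow's direction, retapers all segments by spline distance, and enables Enhanced Input.
; WASD input then rotates the Arrow within limits around the tip's tangent to aim further growth.
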(event `self.ReceiveBeginPlay`
  (bind _returnvalue (`GameplayStatics.GetPlayerController` 0))
  (`|ExecutionSequence`
    (:`then_0`
      (set `self.MaterialInstance` "/Game/GamePlay/Materials/MI_BasicBranch.MI_BasicBranch"))
    (:`then_1`
      (set `PlayerController.bEnableMouseOverEvents` true _returnvalue)
      (set `PlayerController.bEnableClickEvents` true _returnvalue)
      (set `PlayerController.bShowMouseCursor` true _returnvalue)
      (`KismetSystemLibrary.ExecuteConsoleCommand` "show splines" null))))

(event `EnhancedInput|/Game/GamePlay/InputHandler/IA_WASD`
  (params (ActionValue :type "Vector2D Structure") (ElapsedSeconds :type "Float (double-precision)") (TriggeredSeconds :type "Float (double-precision)") (InputAction :type "InputAction Object Reference" :default "/Game/GamePlay/InputHandler/IA_WASD.IA_WASD"))
  (:`Triggered`
    (`self.RotateArrow` ActionValue_X ActionValue_Y)))

(event `OnBranchClicked`
  (params (TouchedComponent :type "PrimitiveComponent Object Reference") (ButtonPressed :type "Key Structure" :default "None"))
  (bind _outactors (`GameplayStatics.GetAllActorsWithTag` "2DCapture"))
  (bind _asbp_scene_capture_2d (cast `/Game/GamePlay/Blueprints/BP_SceneCapture2D` (`|GetArrayItem` _outactors)))
  (`/Game/GamePlay/Blueprints/BP_SceneCapture2D.SetCameraTarget` _asbp_scene_capture_2d self)
  (bind _widget (`/Game/GamePlay/UI/LayerManager/BPFL_UI.PushContentToLayer` (`GameplayStatics.GetPlayerController` 0) (struct :`TagName` "UI.Layer.TreeDetails") "/Game/GamePlay/UI/Menus/UI_TreeDetails/WBP_BsicTreeDetails.WBP_BsicTreeDetails_C"))
  (bind _aswbp_bsic_tree_details (cast `/Game/GamePlay/UI/Menus/UI_TreeDetails/WBP_BsicTreeDetails` _widget))
  (add `/Game/GamePlay/UI/Widgets/UI_BasicElements/WBP_BasicButton.OnCLicked` (`/Game/GamePlay/UI/Menus/UI_TreeDetails/WBP_BsicTreeDetails.BuildButton` _aswbp_bsic_tree_details) (`|CreateDelegate` :!event `ButtonClicked`))
  (bind _hotres (`/Game/GamePlay/UI/Menus/UI_TreeDetails/WBP_BsicTreeDetails.HotRes` _aswbp_bsic_tree_details))
  (`/Game/GamePlay/UI/Widgets/UI_BasicElements/WBP_BasicUpgrater.UpdateProgressBar` _hotres (`self.MaxHotRes`) (`self.ActualHotRes`))
  (add `/Game/GamePlay/UI/Widgets/UI_BasicElements/WBP_BasicUpgrater.OnClicked` _hotres (`|CreateDelegate` :!event `HotResUpdaterClicked`)))

(event `BeginCursorOverBranch`
  (params (TouchedComponent :type "PrimitiveComponent Object Reference"))
  (`KismetSystemLibrary.PrintString` "start")
  (`self.ChangetAllMaterialInstance` "Brightness" 1.0 (`self.BranchPlannerMeshes`)))

(event `EndCursorOverBranch`
  (params (TouchedComponent :type "PrimitiveComponent Object Reference"))
  (`KismetSystemLibrary.PrintString` "end")
  (`self.ChangetAllMaterialInstance` "Brightness" 0.3 (`self.BranchPlannerMeshes`)))

(event `ButtonClicked`
  (params (Button :type "/Game/GamePlay/UI/Widgets/UI_BasicElements/WBP_BasicButton Object Reference"))
  (`self.GrowBranch`)
  (`self.SetSplineScale` (`self.BranchPlannerMeshes`))
  (`self.SetArrowLocation`)
  (`self.AttachControllInputs`))

(event `HotResUpdaterClicked`
  (params (Upgrater :type "/Game/GamePlay/UI/Widgets/UI_BasicElements/WBP_BasicUpgrater Object Reference"))
  (set `self.ActualHotRes` (+ (`self.ActualHotRes`) 10.0))
  (`/Game/GamePlay/UI/Widgets/UI_BasicElements/WBP_BasicUpgrater.UpdateProgressBar` Upgrater (`self.MaxHotRes`) (`self.ActualHotRes`)))

(fn `AddInputBindingToSplineMesh`
  (params (SplineMesh :type "SplineMeshComponent Object Reference"))
  (add `PrimitiveComponent.OnClicked` SplineMesh (`|CreateDelegate` :!event `OnBranchClicked`))
  (add `PrimitiveComponent.OnBeginCursorOver` SplineMesh (`|CreateDelegate` :!event `BeginCursorOverBranch`))
  (add `PrimitiveComponent.OnEndCursorOver` SplineMesh (`|CreateDelegate` :!event `EndCursorOverBranch`)))

(fn `AddMaterialToSplineMesh`
  (params (SplineMesh :type "SplineMeshComponent Object Reference"))
  (`PrimitiveComponent.CreateDynamicMaterialInstance` SplineMesh 0 (`self.MaterialInstance`) "None")
  (`PrimitiveComponent.SetScalarParameterForCustomPrimitiveData` SplineMesh "Brightness" (`self.ActualBrightnessCustomParameter`)))

(fn `AddSplineMesh`
  (bind _branch (`self.Branch`))
  (bind _returnvalue (`SplineComponent.GetNumberOfSplinePoints` (`self.Branch`)))
  (bind _returnvalue_2 (- _returnvalue 2))
  (bind _returnvalue_3 (- _returnvalue 1))
  (bind _returnvalue_4 (`AddComponent|NODE_AddSplineMeshComponent-3`))
  (`KismetArrayLibrary.Array_Add` (`self.BranchPlannerMeshes`) _returnvalue_4)
  (`SplineMeshComponent.SetForwardAxis` _returnvalue_4 "Y" true)
  (`SceneComponent.K2_AttachToComponent` _returnvalue_4 (`self.Branch`) "None" "KeepRelative" "KeepRelative" "KeepRelative" true)
  (bind _spliemeshsizes_x (`KismetMathLibrary.BreakVector` (`self.GetSplineMeshHalfSizes` _returnvalue_4)))
  (`SplineMeshComponent.SetStartAndEnd` _returnvalue_4 (+ (`SplineComponent.GetLocationAtSplinePoint` _branch _returnvalue_2 "Local") (`KismetMathLibrary.MakeVector` 0.0 _spliemeshsizes_x)) (`SplineComponent.GetTangentAtSplinePoint` _branch _returnvalue_2 "Local") (+ (`SplineComponent.GetLocationAtSplinePoint` _branch _returnvalue_3 "Local") (`KismetMathLibrary.MakeVector` 0.0 _spliemeshsizes_x)) (`SplineComponent.GetTangentAtSplinePoint` _branch _returnvalue_3 "Local") true)
  (`self.AddInputBindingToSplineMesh` _returnvalue_4)
  (`self.AddMaterialToSplineMesh` _returnvalue_4))

(fn `AttachControllInputs`
  (`self.EnableInput` (`GameplayStatics.GetPlayerController` 0))
  (bind _asplayer_controller (cast `PlayerController` (`Pawn.GetController` (`GameplayStatics.GetPlayerPawn` 0))))
  (bind _returnvalue (pcsubsystem `EnhancedInputLocalPlayerSubsystem` _asplayer_controller))
  (`/Engine/EditorBlueprintResources/StandardMacros.IsValid` _returnvalue
    (:`Is Valid`
      (`EnhancedInputSubsystemInterface.AddMappingContext` _returnvalue "/Game/GamePlay/InputHandler/IMC_Basic_Iput.IMC_Basic_Iput" 0 (struct)))))

(fn `ChangetAllMaterialInstance`
  (params (ScalarParameterName :type Name) (ParameterValue :type "Float (double-precision)") (BranchMashes :type "Array of SplineMeshComponent Object Reference"))
  (bind _output_get (set `self.ActualBrightnessCustomParameter` ParameterValue))
  (for _array_element BranchMashes
    (`PrimitiveComponent.SetScalarParameterForCustomPrimitiveData` _array_element ScalarParameterName _output_get)))

(fn `CheckRotationValue`
  (params (PitchRotationValue :type "Float (double-precision)") (YawRotationValue :type "Float (double-precision)"))
  (returns (IsValidValues :type Boolean) (ArrowPitchRotationValue :type "Float (double-precision)") (ArrowYawRotationValue :type "Float (double-precision)"))
  (bind (_arrowstartrotation_roll _arrowstartrotation_pitch _arrowstartrotation_yaw) (`KismetMathLibrary.BreakRotator` (`self.ArrowStartRotation`)))
  (bind _minmaxarrowrotationvalue (`self.MinMaxArrowRotationValue`))
  (bind (_arrowstartrotation_roll_2 _arrowstartrotation_pitch_2) (`KismetMathLibrary.BreakRotator` (`self.ArrowStartRotation`)))
  (bind _minmaxarrowrotationvalue_2 (`self.MinMaxArrowRotationValue`))
  (bind _returnvalue (+ (* YawRotationValue (`self.ArrowRotationSpeed`)) (`self.ArrowYawRotationValue`)))
  (bind _returnvalue_2 (+ (* PitchRotationValue (`self.ArrowRotationSpeed`)) (`self.ArrowPitchRotationValue`)))
  (return (and (and (<= _returnvalue (+ _arrowstartrotation_yaw _minmaxarrowrotationvalue)) (>= _returnvalue (- _arrowstartrotation_yaw _minmaxarrowrotationvalue))) (and (<= _returnvalue_2 (+ _arrowstartrotation_pitch_2 _minmaxarrowrotationvalue_2)) (>= _returnvalue_2 (- _arrowstartrotation_pitch_2 _minmaxarrowrotationvalue_2)))) _returnvalue_2 _returnvalue))

(fn `EndBuild`
  (set `self.IsBuildingStarted` false))

(fn `Get Trunk Width`
  (params (Index :type Integer) (SplinePointsNum :type Integer))
  (returns (PointScale :type "Float (double-precision)"))
  (bind _returnvalue (/ (`KismetMathLibrary.MultiplyMultiply_FloatFloat` (* (`SplineComponent.GetDistanceAlongSplineAtSplinePoint` (`self.Branch`) (- SplinePointsNum Index)) 0.2) 0.8) (`KismetMathLibrary.Abs` (`self.BasicStartWidth`))))
  (`KismetSystemLibrary.PrintString` (`KismetStringLibrary.Conv_DoubleToString` _returnvalue))
  (return _returnvalue))

(fn `GetSplineMeshHalfSizes`
  (params (SplineMesh :type "SplineMeshComponent Object Reference"))
  (returns (SplieMeshSizes :type "Vector Structure"))
  (bind (_min _max) (`StaticMeshComponent.GetLocalBounds` SplineMesh))
  (return (/ (- _min _max) (2.0 2.0 2.0))))

(fn `GrowBranch`
  (bind _arrow (`self.Arrow`))
  (`SplineComponent.AddSplinePoint` (`self.Branch`) (+ (`SceneComponent.K2_GetComponentLocation` _arrow) (* (`SceneComponent.GetForwardVector` _arrow) (`ArrowComponent.ArrowLength` _arrow))) "World" true)
  (`self.AddSplineMesh`))

(fn `RotateArrow`
  (params (PitchRotationValue :type "Float (double-precision)") (YawRotationValue :type "Float (double-precision)"))
  (bind (_isvalidvalues _arrowpitchrotationvalue _arrowyawrotationvalue) (`self.CheckRotationValue` PitchRotationValue YawRotationValue))
  (if _isvalidvalues
    (bind _output_get (set `self.ArrowPitchRotationValue` _arrowpitchrotationvalue))
    (bind _output_get_2 (set `self.ArrowYawRotationValue` _arrowyawrotationvalue))
    (`SceneComponent.K2_SetRelativeRotation` (`self.Arrow`) (`KismetMathLibrary.MakeRotator` 0.0 _output_get _output_get_2) false false)))

(fn `SetArrowLocation`
  (bind _branch (`self.Branch`))
  (bind _returnvalue (- (`SplineComponent.GetNumberOfSplinePoints` _branch) 1))
  (bind _returnvalue_2 (`KismetMathLibrary.Conv_VectorToRotator` (`SplineComponent.GetTangentAtSplinePoint` _branch _returnvalue "Local")))
  (`SceneComponent.K2_SetRelativeLocationAndRotation` (`self.Arrow`) (`SplineComponent.GetLocationAtSplinePoint` _branch _returnvalue "Local") _returnvalue_2 false false)
  (set `self.ArrowStartRotation` _returnvalue_2))

(fn `SetSplineScale`
  (params (BranchMeshes :type "Array of SplineMeshComponent Object Reference"))
  (locals (SplinePointsNum :type Integer) (TmpStartScale :type "Float (double-precision)") (TmpEndScale :type "Float (double-precision)"))
  (bind _branch (`self.Branch`))
  (bind _tmpendscale (`local.TmpEndScale`))
  (bind _tmpstartscale (`local.TmpStartScale`))
  (bind _branch_2 (`self.Branch`))
  (bind _output_get (set `local.SplinePointsNum` (`KismetArrayLibrary.Array_Length` BranchMeshes)))
  (set `local.TmpStartScale` (`self.Get Trunk Width` 0 _output_get))
  (set `local.TmpEndScale` (`self.Get Trunk Width` 1 _output_get))
  (for _index (range _output_get)
    (bind _output (`|GetArrayItem` BranchMeshes _index))
    (`SplineMeshComponent.SetStartScale` _output (`KismetMathLibrary.MakeVector2D` _tmpstartscale _tmpstartscale) true)
    (`SplineMeshComponent.SetEndScale` _output (`KismetMathLibrary.MakeVector2D` _tmpendscale _tmpendscale) true)
    (bind _spliemeshsizes_x (`KismetMathLibrary.BreakVector` (`self.GetSplineMeshHalfSizes` _output)))
    (bind _returnvalue (+ _index 1))
    (`SplineMeshComponent.SetStartAndEnd` _output (+ (`SplineComponent.GetLocationAtSplinePoint` _branch_2 _index "Local") (`KismetMathLibrary.MakeVector` 0.0 (* _spliemeshsizes_x (`local.TmpStartScale`)))) (`SplineComponent.GetTangentAtSplinePoint` _branch_2 _index "Local") (+ (`SplineComponent.GetLocationAtSplinePoint` _branch _returnvalue "Local") (`KismetMathLibrary.MakeVector` 0.0 (* _spliemeshsizes_x (`local.TmpEndScale`)))) (`SplineComponent.GetTangentAtSplinePoint` _branch _returnvalue "Local") true)
    (set `local.TmpStartScale` (`local.TmpEndScale`))
    (set `local.TmpEndScale` (`self.Get Trunk Width` _returnvalue (`local.SplinePointsNum`)))))

(fn `StartBuild`
  (set `self.IsBuildingStarted` true))

(fn `UserConstructionScript`
  (locals (SplinePointsNum :type Integer))
  (bind _branch (`self.Branch`))
  (bind _branch_2 (`self.Branch`))
  (bind _startscale (`self.StartScale`))
  (bind _endscale (`self.EndScale`))
  (bind _returnvalue (`SplineComponent.GetNumberOfSplinePoints` (`self.Branch`)))
  (set `self.MaterialInstance` "/Game/GamePlay/Materials/MI_BasicBranch.MI_BasicBranch")
  (set `local.SplinePointsNum` _returnvalue)
  (for _index (range (+ (- _returnvalue 2) 1))
    (bind _returnvalue_2 (`AddComponent|NODE_AddSplineMeshComponent-2`))
    (`KismetArrayLibrary.Array_Add` (`self.BranchPlannerMeshes`) _returnvalue_2)
    (`SplineMeshComponent.SetForwardAxis` _returnvalue_2 "Y" true)
    (`SceneComponent.K2_AttachToComponent` _returnvalue_2 (`self.Branch`) "None" "KeepRelative" "KeepRelative" "KeepRelative" true)
    (bind _spliemeshsizes_x (`KismetMathLibrary.BreakVector` (`self.GetSplineMeshHalfSizes` _returnvalue_2)))
    (bind _returnvalue_3 (+ _index 1))
    (`SplineMeshComponent.SetStartAndEnd` _returnvalue_2 (+ (`SplineComponent.GetLocationAtSplinePoint` _branch_2 _index "Local") (`KismetMathLibrary.MakeVector` 0.0 (* _spliemeshsizes_x (`self.StartScale`)))) (`SplineComponent.GetTangentAtSplinePoint` _branch_2 _index "Local") (+ (`SplineComponent.GetLocationAtSplinePoint` _branch _returnvalue_3 "Local") (`KismetMathLibrary.MakeVector` 0.0 (* _spliemeshsizes_x (`self.EndScale`)))) (`SplineComponent.GetTangentAtSplinePoint` _branch _returnvalue_3 "Local") true)
    (`SplineMeshComponent.SetEndScale` _returnvalue_2 (`KismetMathLibrary.MakeVector2D` _endscale _endscale) true)
    (`SplineMeshComponent.SetStartScale` _returnvalue_2 (`KismetMathLibrary.MakeVector2D` _startscale _startscale) true)
    (bind (_min _max) (`StaticMeshComponent.GetLocalBounds` _returnvalue_2))
    (bind _returnvalue_x (`KismetMathLibrary.BreakVector` (- _min _max)))
    (set `self.BasicStartWidth` _returnvalue_x)
    (`self.AddInputBindingToSplineMesh` _returnvalue_2)
    (`self.AddMaterialToSplineMesh` _returnvalue_2)
    (`self.SetArrowLocation`)))