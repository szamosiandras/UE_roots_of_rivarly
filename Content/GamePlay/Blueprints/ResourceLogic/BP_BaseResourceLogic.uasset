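; Base Blueprint for a game resource that tracks amount, capacity and summed income.
; On BeginPlay it binds to the environment time tick in BP_GamePLayGameState, adding income on each tick instead of using Tick.
; Income and manual additions clamp the amount to capacity, then CheckResource runs ResourceLogic, here only a debug print, and broadcasts the fill ratio for UI updates.
; Setup, increment and getter functions expose the values.
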(event `self.ReceiveBeginPlay`
  (`self.BindEventToEnvironmentTick`))

(event `EnvironmentTImeTick`
  (params (Time :type Integer))
  (`self.CalculateResourceIncome`))

(fn `AddAmoutToResource`
  (params (Amount :type "Float (double-precision)"))
  (locals (TmpAmount :type "Float (double-precision)"))
  (set `local.TmpAmount` Amount)
  (set `self.ResourceAmount` (`KismetMathLibrary.FClamp` (+ (`local.TmpAmount`) (`self.ResourceAmount`)) 0.0 (`self.ResourceCapacity`)))
  (`self.CheckResource`))

(fn `AddResourceCapacity`
  (params (AddResourceCapacity :type "Float (double-precision)"))
  (set `self.ResourceCapacity` (+ AddResourceCapacity (`self.ResourceCapacity`))))

(fn `AddResourceSummIncome`
  (params (AddResourceSummIncome :type "Float (double-precision)"))
  (set `self.ResourceSummIncome` (+ AddResourceSummIncome (`self.ResourceSummIncome`))))

(fn `BindEventToEnvironmentTick`
  (bind _asbp_game_play_game_state (cast `/Game/GamePlay/Core/BP_GamePLayGameState` (`GameplayStatics.GetGameState`)))
  (add `/Game/GamePlay/Core/BP_GamePLayGameState.EnvironmentTimeTick` _asbp_game_play_game_state (`|CreateDelegate` :!event `EnvironmentTImeTick`)))

(fn `CalculateResourceIncome`
  (returns (ResourceIncome :type "Float (double-precision)"))
  (set `self.ResourceAmount` (`KismetMathLibrary.FClamp` (+ (`self.ResourceAmount`) (`self.ResourceSummIncome`)) 0.0 (`self.ResourceCapacity`)))
  (`self.CheckResource`)
  (return (`self.ResourceSummIncome`)))

(fn `CheckResource`
  (`self.ResourceLogic`)
  (`self.UpdateUI`))

(fn `GetResourceAmount`
  (returns (ResourceAmount :type "Float (double-precision)"))
  (return (`self.ResourceAmount`)))

(fn `GetResourceCapacity`
  (returns (ResourceCapacity :type "Float (double-precision)"))
  (return (`self.ResourceCapacity`)))

(fn `GetResourceSummIncome`
  (returns (ResourceSummIncome :type "Float (double-precision)"))
  (return (`self.ResourceSummIncome`)))

(fn `GetResourceValue`
  (returns (ResourceValue :type "Float (double-precision)"))
  (return (/ (`self.ResourceAmount`) (`self.ResourceCapacity`))))

(fn `ResourceInit`
  (params (ResourceCapacity :type "Float (double-precision)") (ResourceSummIncome :type "Float (double-precision)") (ResourceAmount :type "Float (double-precision)"))
  (set `self.ResourceCapacity` ResourceCapacity)
  (set `self.ResourceSummIncome` ResourceSummIncome)
  (set `self.ResourceAmount` ResourceAmount))

(fn `ResourceLogic`
  (`KismetSystemLibrary.PrintString` "ResourceLogic"))

(fn `UpdateUI`
  (`self.UpdateResourceUI` (`self.GetResourceValue`)))