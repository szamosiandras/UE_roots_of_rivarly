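; Health resource logic Blueprint, a child resource class that applies health change amounts to its resource total.
; BindHealthAmountChange binds an event to the health-change binding on the game state's EnergyLogic, linking health to the energy resource logic.
; The HealthChange event passes its amount to AddAmoutToResource.
; ResourceLogic only prints a debug string, and UpdateUI prints before calling the parent version.
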(event `self.ReceiveBeginPlay`
  (`parent.ReceiveBeginPlay`))

(event `HealthChange`
  (params (HealthChangeAmount :type "Float (double-precision)"))
  (`self.AddAmoutToResource` HealthChangeAmount))

(fn `BindHealthAmountChange`
  (bind _asbp_game_play_game_state (cast `/Game/GamePlay/Core/BP_GamePLayGameState` (`GameplayStatics.GetGameState`)))
  (add `/Game/GamePlay/Blueprints/ResourceLogic/BP_EnergyLogic.ChangeHealtAmount` (`/Game/GamePlay/Core/BP_GamePLayGameState.EnergyLogic` _asbp_game_play_game_state) (`|CreateDelegate` :!event `HealthChange`)))

(fn `ResourceLogic`
  (`KismetSystemLibrary.PrintString` "HEALTH LOGIC"))

(fn `UpdateUI`
  (`KismetSystemLibrary.PrintString` "UPDATE HEALTH")
  (`parent.UpdateUI`))