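; BP_CameraControler is a camera controller actor that pans across the world by mouse drag.
; BeginPlay shows the cursor, enables touch events and prints a debug string.
; The DragCamera press stores the viewport mouse position, then Tick, while the key is held, offsets the actor horizontally by the frame-to-frame pointer delta.
; Screen Y maps to world X and negated screen X to world Y, unscaled and without sweep.
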(event `self.ReceiveBeginPlay`
  (bind _returnvalue (`GameplayStatics.GetPlayerController` 0))
  (set `PlayerController.bShowMouseCursor` true _returnvalue)
  (set `PlayerController.bEnableTouchEvents` true _returnvalue)
  (`KismetSystemLibrary.PrintString` "haloooooooooooooooooooooooooo"))

(event `InputAction|DragCamera`
  (params (Key :type "Key Structure"))
  (:`Pressed`
    (bind _returnvalue (`WidgetLayoutLibrary.GetMousePositionOnViewport`))
    (set `self.PreviousTouchLocation` _returnvalue)))

(event `self.ReceiveTick`
  (params (DeltaSeconds :type "Float (single-precision)"))
  (bind (_returnvalue_x _returnvalue_y) (`KismetMathLibrary.BreakVector2D` (- (`self.NewTouchLocation`) (`self.PreviousTouchLocation`))))
  (if (`PlayerController.IsInputKeyDown` (`GameplayStatics.GetPlayerController` 0) (stale `InputAction|DragCamera` Key))
    (bind _returnvalue (`WidgetLayoutLibrary.GetMousePositionOnViewport`))
    (set `self.NewTouchLocation` _returnvalue)
    (`self.K2_AddActorWorldOffset` (`KismetMathLibrary.MakeVector` _returnvalue_y (* _returnvalue_x -1.0)))
    (set `self.PreviousTouchLocation` (`self.NewTouchLocation`))))

(fn `UserConstructionScript`)