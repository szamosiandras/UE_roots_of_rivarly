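; Game state that keeps the gameplay clock and the player's Health, Energy and Nutrient resources.
; A looping one-second timer increments Time and passes it to CallEnvironmentTimeTick; BeginPlay also binds HealthLogic to health changes.
; UpdatePlayerResources, not called within this graph, applies clamped incomes and refreshes the main widget's bars.
; AddHealthPoint adds health unclamped, HealthToEnergy scales energy income to the health range, and AddNutrient is an empty stub.
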(event `self.ReceiveBeginPlay`
  (`KismetSystemLibrary.K2_SetTimerDelegate` (delegate `TimeTick`) 1.0 true)
  (`/Game/GamePlay/Blueprints/ResourceLogic/BP_HealthResourceLogic.BindHealthAmountChange` (`self.HealthLogic`)))

(event `TimeTick`
  (bind _result (`/Engine/EditorBlueprintResources/StandardMacros.IncrementInt` (`self.Time`))
    (:`  `
      (`KismetSystemLibrary.PrintString` (`KismetStringLibrary.Conv_IntToString` _result))
      (`self.EnvironmentTimeTick` self (`self.Time`)))))

(fn `AddAmountToResource`
  (params (Resource :type "/Game/GamePlay/Blueprints/ResourceLogic/ResourceStruct Structure (by ref)") (Amount :type "Float (double-precision)"))
  (bind (_maxamount _incomeamount _amount) (break `/Game/GamePlay/Blueprints/ResourceLogic/ResourceStruct` Resource))
  (`|VariableSetRef` Resource (make `/Game/GamePlay/Blueprints/ResourceLogic/ResourceStruct` _maxamount _incomeamount (+ Amount _amount))))

(fn `AddHealthPoint`
  (params (IncomeAmount :type "Float (double-precision)"))
  (`self.AddAmountToResource` (`self.HealthPoint`) IncomeAmount)
  (`self.UpdateHealthBar`))

(fn `AddNutrient`)

(fn `CalculateResourceIncome`
  (params (Resource :type "/Game/GamePlay/Blueprints/ResourceLogic/ResourceStruct Structure (by ref)"))
  (returns (Income :type "Float (double-precision)"))
  (bind (_maxamount _incomeamount _amount) (break `/Game/GamePlay/Blueprints/ResourceLogic/ResourceStruct` Resource))
  (`|VariableSetRef` Resource (make `/Game/GamePlay/Blueprints/ResourceLogic/ResourceStruct` _maxamount _incomeamount (`KismetMathLibrary.FClamp` (+ _amount _incomeamount) 0.0 _maxamount)))
  (return _incomeamount))

(fn `GetValueOfResource`
  (params (Resource :type "/Game/GamePlay/Blueprints/ResourceLogic/ResourceStruct Structure"))
  (returns (ResourceValue :type "Float (double-precision)"))
  (return (/ Resource_Amount_3_C9ADC3F045A1A51970B402B2977BC7C7 Resource_MaxAmount_5_83803DD1441277A35205A680434DD48C)))

(fn `HealthToEnergy`
  (params (EnergyIncome :type "Float (double-precision)"))
  (returns (HealthLoss :type "Float (double-precision)"))
  (return (* (`.MaxAmount_5_83803DD1441277A35205A680434DD48C` (break `/Game/GamePlay/Blueprints/ResourceLogic/ResourceStruct` (`self.HealthPoint`))) (/ EnergyIncome (`.MaxAmount_5_83803DD1441277A35205A680434DD48C` (break `/Game/GamePlay/Blueprints/ResourceLogic/ResourceStruct` (`self.Energy`)))))))

(fn `UpdateEnergyBar`
  (bind _maingameplaywidget (`/Game/GamePlay/UI/LayerManager/BPFL_UI.GetMainGamePlayWidget`))
  (`/Game/GamePlay/UI/Menus/UI_MainGameplay/WBP_MainGamePLay.UpdateEnergyBar` _maingameplaywidget (`self.GetValueOfResource` (`self.Energy`))))

(fn `UpdateHealthBar`
  (bind _maingameplaywidget (`/Game/GamePlay/UI/LayerManager/BPFL_UI.GetMainGamePlayWidget`))
  (`/Game/GamePlay/UI/Menus/UI_MainGameplay/WBP_MainGamePLay.UpdateHealthBar` _maingameplaywidget (`self.GetValueOfResource` (`self.HealthPoint`))))

(fn `UpdateIncomes`
  (`self.CalculateResourceIncome` (`self.HealthPoint`))
  (`self.CalculateResourceIncome` (`self.Energy`))
  (`self.CalculateResourceIncome` (`self.Nutrient`)))

(fn `UpdateNutrientBar`
  (bind _maingameplaywidget (`/Game/GamePlay/UI/LayerManager/BPFL_UI.GetMainGamePlayWidget`))
  (`/Game/GamePlay/UI/Menus/UI_MainGameplay/WBP_MainGamePLay.UpdateNutrientBar` _maingameplaywidget (`self.GetValueOfResource` (`self.Nutrient`))))

(fn `UpdatePlayerResources`
  (`self.UpdateIncomes`)
  (`self.UpdateProgressBars`))

(fn `UpdateProgressBars`
  (`self.UpdateNutrientBar`)
  (`self.UpdateEnergyBar`)
  (`self.UpdateHealthBar`))

(fn `UserConstructionScript`)