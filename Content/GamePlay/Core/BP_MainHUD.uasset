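; BP_MainHUD is the game's main HUD, which owns the root layered UI layout.
; On BeginPlay it creates WBP_PrimaryLayout with its initial screens, adds it to the viewport, pops the TreeDetails layer and updates player resources.
; Its functions wrap the layout's layer API to register, push, pop, clear and query layers by name or tag, serving as a single access point for UI stacking.
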(event `self.ReceiveBeginPlay`
  (bind _returnvalue (`|CreateWidget` "/Game/GamePlay/UI/LayerManager/WBP_PrimaryLayout.WBP_PrimaryLayout_C" (`self.GetOwningPlayerController`) (`self.InitialScreens`)))
  (set `self.PrimaryLayout` _returnvalue)
  (`UserWidget.AddToViewport` _returnvalue 0)
  (`self.PopContentFromLayer` (struct :`TagName` "UI.Layer.TreeDetails"))
  (`/Game/GamePlay/UI/LayerManager/BPFL_UI.UpdatePlayerResources`))

(fn `ClearAllLayers`
  (`/Game/GamePlay/UI/LayerManager/WBP_PrimaryLayout.ClearAllLayers` (`self.GetPrimaryLayout`)))

(fn `ClearAllLayersExcept`
  (params (LayerName :type "GameplayTag Structure"))
  (`/Game/GamePlay/UI/LayerManager/WBP_PrimaryLayout.ClearAllLayersExcept` (`self.GetPrimaryLayout`) LayerName))

(fn `ClearLayer`
  (params (LayerName :type "GameplayTag Structure"))
  (`/Game/GamePlay/UI/LayerManager/WBP_PrimaryLayout.ClearLayer` (`self.GetPrimaryLayout`) LayerName))

(fn `GetLayerByTag`
  (params (LayerName :type "GameplayTag Structure"))
  (returns (IsLayerAvailable :type Boolean) (TopWidgetByTag :type "UserWidget Object Reference"))
  (bind (_islayeravailable _topwidgetbytag) (`/Game/GamePlay/UI/LayerManager/WBP_PrimaryLayout.GetLayerByTag` (`self.PrimaryLayout`) LayerName))
  (return _islayeravailable _topwidgetbytag))

(fn `GetPrimaryLayout`
  (returns (PrymaryLayout :type "/Game/GamePlay/UI/LayerManager/WBP_PrimaryLayout Object Reference"))
  (return (`self.PrimaryLayout`)))

(fn `PopContentFromLayer`
  (params (LayerName :type "GameplayTag Structure"))
  (`/Game/GamePlay/UI/LayerManager/WBP_PrimaryLayout.PopContentFromLayer` (`self.GetPrimaryLayout`) LayerName)
  (return))

(fn `PushContentToLayer`
  (params (LayerName :type "GameplayTag Structure") (UserWidget :type "UserWidget Soft Class Reference"))
  (returns (ReturnValue :type "UserWidget Object Reference"))
  (bind _newparam (`/Game/GamePlay/UI/LayerManager/WBP_PrimaryLayout.PushContentToLayer` (`self.GetPrimaryLayout`) LayerName UserWidget))
  (return _newparam))

(fn `RegisterLayer`
  (params (LayerName :type "GameplayTag Structure") (LayerWidget :type "/Game/GamePlay/UI/LayerManager/WBP_Layer Object Reference"))
  (returns (ReturnValue :type Boolean))
  (bind _returnvalue (`/Game/GamePlay/UI/LayerManager/WBP_PrimaryLayout.RegisterLayer` (`self.GetPrimaryLayout`) LayerName LayerWidget))
  (return _returnvalue))

(fn `UnRegisterLayer`
  (params (`Layer Name` :type "GameplayTag Structure"))
  (returns (ReturnValue :type Boolean))
  (bind _returnvalue (`/Game/GamePlay/UI/LayerManager/WBP_PrimaryLayout.UnRegisterLayer` (`self.GetPrimaryLayout`) `Layer Name`))
  (return _returnvalue))

(fn `UserConstructionScript`)