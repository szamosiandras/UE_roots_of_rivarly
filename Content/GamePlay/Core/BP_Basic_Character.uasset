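; Player character acting as a camera rig with tree, surrounding and root views; it spawns a BP_BranchFactory as MainTree on BeginPlay.
; View switches save and reload transform and spring arm length through per-view structs, whose active flags also route Enhanced Input to panning, orbiting or looking.
; The mouse wheel zooms the spring arm above a minimum length.
; Camera widget setup and grid cursor selection are disconnected, leaving the Tick cursor update empty.
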(event `self.ReceiveBeginPlay`
  ;[1 1 1] Setup Controlls
  (bind _asplayer_controller (cast `PlayerController` (`self.GetController`)))
  (bind _returnvalue (pcsubsystem `EnhancedInputLocalPlayerSubsystem` _asplayer_controller))
  (`/Engine/EditorBlueprintResources/StandardMacros.IsValid` _returnvalue
    (:`Is Valid`
      (`EnhancedInputSubsystemInterface.AddMappingContext` _returnvalue "/Game/GamePlay/InputHandler/IMC_Basic_Iput.IMC_Basic_Iput" 0 (struct))
      (bind _returnvalue_2 (`|SpawnActorFromClass` "/Game/GamePlay/Blueprints/BP_BranchFactory.BP_BranchFactory_C" (`KismetMathLibrary.MakeTransform` (0.0 0.0 0.0) (struct :`Pitch` 90.0)) "AlwaysSpawn" "MultiplyWithRoot" null null))
      (`/Engine/EditorBlueprintResources/StandardMacros.IsValid` _returnvalue_2
        (:`Is Valid`
          (set `self.MainTree` _returnvalue_2))))))

(event `EnhancedInput|/Game/GamePlay/InputHandler/IA_WASD`
  (params (ActionValue :type "Vector2D Structure") (ElapsedSeconds :type "Float (double-precision)") (TriggeredSeconds :type "Float (double-precision)") (InputAction :type "InputAction Object Reference" :default "/Game/GamePlay/InputHandler/IA_WASD.IA_WASD"))
  ;[1 1 1] WASD controll
  (:`Triggered`
    (`self.Actions_WASD` ActionValue_X ActionValue_Y)))

(event `EnhancedInput|/Game/GamePlay/InputHandler/IA_Mouse`
  (params (ActionValue :type "Vector2D Structure") (ElapsedSeconds :type "Float (double-precision)") (TriggeredSeconds :type "Float (double-precision)") (InputAction :type "InputAction Object Reference" :default "/Game/GamePlay/InputHandler/IA_Mouse.IA_Mouse"))
  ;[1 1 1] Mouse Controll
  (:`Triggered`
    (`self.Actions_Mouse` ActionValue_X ActionValue_Y)))

(event `EnhancedInput|/Game/GamePlay/InputHandler/IA_MouseWheel`
  (params (ActionValue :type "Float (double-precision)") (ElapsedSeconds :type "Float (double-precision)") (TriggeredSeconds :type "Float (double-precision)") (InputAction :type "InputAction Object Reference" :default "/Game/GamePlay/InputHandler/IA_MouseWheel.IA_MouseWheel"))
  (:`Triggered`
    (`self.Actions_MouseWheel` ActionValue)))

(event `self.ReceiveTick`
  (params (DeltaSeconds :type "Float (single-precision)"))
  (`self.UpdateCursorPosition`))

(fn `Actions_Mouse`
  (params (X :type "Float (double-precision)") (Y :type "Float (double-precision)"))
  (bind _returnvalue (* Y 10.0))
  (if (`.IsCameraActive_6_EB09672A4034881512CB6099199764F2` (break `/Game/GamePlay/Core/S_CameraViewDatas` (`self.CameraParameters_Surrounding`)))
    (`self.K2_AddActorWorldOffset` (`KismetMathLibrary.MakeVector` _returnvalue (* X -10.0)))
    (elif (`.IsCameraActive_6_EB09672A4034881512CB6099199764F2` (break `/Game/GamePlay/Core/S_CameraViewDatas` (`self.CameraParameters_Tree`)))
      (`self.K2_AddActorWorldRotation` (`KismetMathLibrary.MakeRotator` 0.0 0.0 (* X 10.0)))
      (`self.K2_AddActorWorldOffset` (`KismetMathLibrary.MakeVector` 0.0 0.0 _returnvalue))
      (elif (`.IsCameraActive_6_EB09672A4034881512CB6099199764F2` (break `/Game/GamePlay/Core/S_CameraViewDatas` (`self.CameraParameters_Root`)))
        (`self.AddControllerYawInput` X)
        (`self.AddControllerPitchInput` Y)))))

(fn `Actions_MouseWheel`
  (params (MouseWheel_x :type "Float (double-precision) (by ref)"))
  (bind _springarm (`self.SpringArm`))
  (bind _returnvalue (+ (`SpringArmComponent.TargetArmLength` _springarm) (* MouseWheel_x 10.0)))
  (if (< 20.0 _returnvalue)
    (set `SpringArmComponent.TargetArmLength` _returnvalue _springarm)))

(fn `Actions_WASD`
  (params (X :type "Float (double-precision)") (Y :type "Float (double-precision)"))
  (bind _returnvalue (* Y 10.0))
  (bind _returnvalue_2 (* X 10.0))
  (if (`.IsCameraActive_6_EB09672A4034881512CB6099199764F2` (break `/Game/GamePlay/Core/S_CameraViewDatas` (`self.CameraParameters_Surrounding`)))
    (`self.K2_AddActorWorldOffset` (`KismetMathLibrary.MakeVector` _returnvalue _returnvalue_2))
    (`KismetSystemLibrary.PrintString` "surr WASD")
    (elif (`.IsCameraActive_6_EB09672A4034881512CB6099199764F2` (break `/Game/GamePlay/Core/S_CameraViewDatas` (`self.CameraParameters_Tree`)))
      (`self.K2_AddActorWorldRotation` (`KismetMathLibrary.MakeRotator` 0.0 0.0 _returnvalue_2))
      (`self.K2_AddActorWorldOffset` (`KismetMathLibrary.MakeVector` 0.0 0.0 _returnvalue))
      (`KismetSystemLibrary.PrintString` "treee wasd")
      (elif (`.IsCameraActive_6_EB09672A4034881512CB6099199764F2` (break `/Game/GamePlay/Core/S_CameraViewDatas` (`self.CameraParameters_Root`)))
        _))))

(fn `Camera_RootView`
  (`self.SaveCameraParameters`)
  (setmembers `/Game/GamePlay/Core/S_CameraViewDatas` :`StructRef` (`self.CameraParameters_Root`) :`IsCameraActive` true)
  (`self.LoadCameraParameters`))

(fn `Camera_SurroundingView`
  (`self.SaveCameraParameters`)
  (setmembers `/Game/GamePlay/Core/S_CameraViewDatas` :`StructRef` (`self.CameraParameters_Surrounding`) :`IsCameraActive` true)
  (`self.LoadCameraParameters`))

(fn `Camera_TreeView`
  (`self.SaveCameraParameters`)
  (setmembers `/Game/GamePlay/Core/S_CameraViewDatas` :`StructRef` (`self.CameraParameters_Tree`) :`IsCameraActive` true)
  (`self.LoadCameraParameters`))

(fn `LoadCameraParameters`
  (if (`.IsCameraActive_6_EB09672A4034881512CB6099199764F2` (break `/Game/GamePlay/Core/S_CameraViewDatas` (`self.CameraParameters_Surrounding`)))
    (`self.LoadCameraView` (`self.CameraParameters_Surrounding`))
    (elif (`.IsCameraActive_6_EB09672A4034881512CB6099199764F2` (break `/Game/GamePlay/Core/S_CameraViewDatas` (`self.CameraParameters_Tree`)))
      (`self.LoadCameraView` (`self.CameraParameters_Tree`))
      (else
        (`self.LoadCameraView` (`self.CameraParameters_Root`))))))

(fn `LoadCameraView`
  (params (CameraViewParameteres :type "/Game/GamePlay/Core/S_CameraViewDatas Structure (by ref)"))
  (bind (_iscameraactive _springarmlength _rotationvector _springarmrotationvector _positionverctor) (break `/Game/GamePlay/Core/S_CameraViewDatas` CameraViewParameteres))
  (bind _springarm (`self.SpringArm`))
  (set `SpringArmComponent.TargetArmLength` _springarmlength _springarm)
  (`self.K2_SetActorRotation` _rotationvector)
  (`SceneComponent.K2_SetWorldRotation` _springarm _springarmrotationvector false false)
  (`self.K2_SetActorLocation` _positionverctor))

(fn `SaveCameraParameters`
  (if (`.IsCameraActive_6_EB09672A4034881512CB6099199764F2` (break `/Game/GamePlay/Core/S_CameraViewDatas` (`self.CameraParameters_Surrounding`)))
    (`self.SaveCameraView` (`self.CameraParameters_Surrounding`))
    (elif (`.IsCameraActive_6_EB09672A4034881512CB6099199764F2` (break `/Game/GamePlay/Core/S_CameraViewDatas` (`self.CameraParameters_Tree`)))
      (`self.SaveCameraView` (`self.CameraParameters_Tree`))
      (else
        (`self.SaveCameraView` (`self.CameraParameters_Root`))))))

(fn `SaveCameraView`
  (params (CameraViewParameteres :type "/Game/GamePlay/Core/S_CameraViewDatas Structure (by ref)"))
  (bind _structout (setmembers `/Game/GamePlay/Core/S_CameraViewDatas` :`StructRef` CameraViewParameteres :`IsCameraActive` false :`SpringArmLength` (`SpringArmComponent.TargetArmLength` (`self.SpringArm`)) :`RotationVector` (`self.K2_GetActorRotation`) :`PositionVerctor` (`self.K2_GetActorLocation`)))
  (setmembers `/Game/GamePlay/Core/S_CameraViewDatas` :`StructRef` _structout :`IsCameraActive` false))

(fn `SetMiddleOfMainTree`
  (bind (_returnvalue_x _returnvalue_y _returnvalue_z) (`KismetMathLibrary.BreakVector` (`self.K2_GetActorLocation` (`self.MainTree`))))
  (`SceneComponent.K2_SetWorldLocation` (`self.CapsuleComponent`) (`KismetMathLibrary.MakeVector` _returnvalue_x _returnvalue_y (+ _returnvalue_z 20.0)) false false))

(fn `UpdateCursorPosition`
  (locals (Grid :type "/Game/GamePlay/Blueprints/Grid/BP_Grid Object Reference") (HitLocation :type "Vector Structure" :default (0.0 0.0 0.0))))

(fn `UserConstructionScript`)